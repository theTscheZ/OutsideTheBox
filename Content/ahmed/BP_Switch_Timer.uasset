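; BP_Switch_Timer is an interactable switch that toggles a set of linked Lamps; despite its name, the graph contains no timer logic.
; Interact uses a FlipFlop to alternate the switch's IsOn flag, while both branches invert each lamp's own IsLightOn, so mixed lamp states stay mixed.
; It then calls SetLight on every lamp to apply the new state.
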(event EventBeginPlay
  (|CallParentFunction) ; This node is disabled and will not be called.\nDrag off pins to build functionality.
)

(event Collision|EventActorBeginOverlap
  (params (OtherActor :type Actor%20Object%20Reference))
  (|CallParentFunction OtherActor) ; This node is disabled and will not be called.\nDrag off pins to build functionality.
)

(event EventTick
  (params (DeltaSeconds :type Float%20%28single-precision%29))
  (|CallParentFunction DeltaSeconds) ; This node is disabled and will not be called.\nDrag off pins to build functionality.
)

(event EventInteract
  (params (Interacting%20Player :type BP%20First%20Person%20Character%20Object%20Reference))
  (bind _lamps (Variables|Default|GetLamps))
  (Utilities|FlowControl|FlipFlop
    (:A
      (Variables|Default|SetIsOn? true)
      (for _array_element _lamps
        (if (Variables|/Game/Interactables/Blueprints/Light/BP_ToggleLight.BP_ToggleLight_C|GetIsLightOn? _array_element)
          (Variables|/Game/Interactables/Blueprints/Light/BP_ToggleLight.BP_ToggleLight_C|SetIsLightOn? _array_element false)
          (else
            (Variables|/Game/Interactables/Blueprints/Light/BP_ToggleLight.BP_ToggleLight_C|SetIsLightOn? _array_element true)))))
    (:B
      (Variables|Default|SetIsOn? false)
      (for _array_element_2 _lamps
        (if (Variables|/Game/Interactables/Blueprints/Light/BP_ToggleLight.BP_ToggleLight_C|GetIsLightOn? _array_element_2)
          (Variables|/Game/Interactables/Blueprints/Light/BP_ToggleLight.BP_ToggleLight_C|SetIsLightOn? _array_element_2 false)
          (else
            (Variables|/Game/Interactables/Blueprints/Light/BP_ToggleLight.BP_ToggleLight_C|SetIsLightOn? _array_element_2 true))))))
  (for _array_element_3 (Variables|Default|GetLamps)
    (Default|SetLight _array_element_3)))

(fn ConstructionScript
  (|CallParentFunction))