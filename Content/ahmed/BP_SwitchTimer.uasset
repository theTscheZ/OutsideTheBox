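; BP_SwitchTimer is an interactable timed switch that temporarily flips a set of lamps.
; Interact calls Licht, waits for the Delay variable, then calls Licht again to flip the lamps back.
; Licht inverts IsLightOn on each entry in Lamps individually and calls its SetLight.
; Interacting again during the wait toggles immediately without queuing another revert, as nothing guards re-entry.
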(event EventBeginPlay
  (|CallParentFunction) ; This node is disabled and will not be called.\nDrag off pins to build functionality.
)

(event Collision|EventActorBeginOverlap
  (params (OtherActor :type Actor%20Object%20Reference))
  (|CallParentFunction OtherActor) ; This node is disabled and will not be called.\nDrag off pins to build functionality.
)

(event EventTick
  (params (DeltaSeconds :type Float%20%28single-precision%29))
  (|CallParentFunction DeltaSeconds) ; This node is disabled and will not be called.\nDrag off pins to build functionality.
)

(event EventInteract
  (params (Interacting%20Player :type BP%20First%20Person%20Character%20Object%20Reference))
  (CallFunction|Licht)
  (Utilities|FlowControl|Delay (Variables|Default|Getdelay))
  (CallFunction|Licht))

(fn ConstructionScript
  (|CallParentFunction))

(fn Licht
  (for _array_element (Variables|Default|GetLamps)
    (if (Variables|/Game/Interactables/Blueprints/Light/BP_ToggleLight.BP_ToggleLight_C|GetIsLightOn? _array_element)
      (Variables|/Game/Interactables/Blueprints/Light/BP_ToggleLight.BP_ToggleLight_C|SetIsLightOn? _array_element false)
      (else
        (Variables|/Game/Interactables/Blueprints/Light/BP_ToggleLight.BP_ToggleLight_C|SetIsLightOn? _array_element true)))
    (Default|SetLight _array_element)))