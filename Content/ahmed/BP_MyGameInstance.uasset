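; Game instance that keeps a usage count for interactable objects, identified by ObjektID.
; UpdateUsageData searches the TrackedObjects array, rewrites a matching entry with its count incremented, or appends a new entry starting at one.
; Increments also print the ID and counts as debug output.
; NewFunction is an unfinished stub with an unconnected struct constructor.
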(fn UpdateUsageData
  (params (ObjektID%20 :type String))
  (for (_array_element _array_index) (Variables|Default|GetTrackedObjects%20)
    (if (Utilities|Enum|Equal(Enum) ObjektID%20 (.ObjektID (Utilities|Struct|BreakBP_InteractableData _array_element)))
      (Utilities|Array|SetArrayElem (Variables|Default|GetTrackedObjects%20) _array_index (Utilities|Struct|MakeBP_InteractableData (.ObjektID (Utilities|Struct|BreakBP_InteractableData _array_element)) (+ (.UsageCount (Utilities|Struct|BreakBP_InteractableData _array_element)) 1)))
      (Development|PrintString "begin")
      (Development|PrintString ObjektID%20)
      (Development|PrintString (Utilities|String|ToString(Integer) (.UsageCount (Utilities|Struct|BreakBP_InteractableData _array_element))))
      (Development|PrintString "new")
      (Development|PrintString (Utilities|String|ToString(Integer) (+ (.UsageCount (Utilities|Struct|BreakBP_InteractableData _array_element)) 1)))
      (Development|PrintString "end")
      (return)))
  (Utilities|Array|Add (Variables|Default|GetTrackedObjects%20) (Utilities|Struct|MakeBP_InteractableData ObjektID%20 1)))

(fn NewFunction
  (params (ObjektID :type String) (UsageCount :type Integer)))