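; BP_Gate is a gate actor that swings its door open when every linked Light is on and closes it otherwise.
; It registers itself on each Light during construction and BeginPlay, running CheckLight at BeginPlay.
; CheckLight counts lit entries against the array's last index, then plays or reverses a Timeline that drives door yaw.
; A level-loading function also exists, but its only call here is in unreachable nodes.
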(event Custom|open
  (bind _door (Timeline|Timeline Play)
    (:Update
      (Transformation|SetRelativeRotation (Variables|Default|Getdoor) (Math|Rotator|MakeRotator 0.0 0.0 (Math|Float|Lerp 0.0 -9e+01 _door)) false false))))

(event Custom|close
  (bind _door (Timeline|Timeline Reverse)
    (:Update
      (Transformation|SetRelativeRotation (Variables|Default|Getdoor) (Math|Rotator|MakeRotator 0.0 0.0 (Math|Float|Lerp 0.0 -9e+01 _door)) false false))))

(event EventBeginPlay
  (for _array_element (Variables|Default|GetLight)
    (Variables|/Game/Interactables/Blueprints/Light/BP_ToggleLight.BP_ToggleLight_C|SetGate _array_element self)
    (CallFunction|CheckLight)))

(event Collision|EventActorBeginOverlap
  (params (OtherActor :type Actor%20Object%20Reference)))

(event EventTick
  (params (DeltaSeconds :type Float%20%28single-precision%29)))

(fn ConstructionScript
  (for _array_element (Variables|Default|GetLight)
    (Variables|/Game/Interactables/Blueprints/Light/BP_ToggleLight.BP_ToggleLight_C|SetGate _array_element self)))

(fn CheckLight
  (bind _light (Variables|Default|GetLight))
  (Variables|Default|SetCounter -1)
  (bind _array_element (Utilities|Array|ForEachLoopwithBreak _light)
    (:LoopBody
      (if (Variables|/Game/Interactables/Blueprints/Light/BP_ToggleLight.BP_ToggleLight_C|GetIsLightOn? _array_element)
        (Math|Integer|IncrementInt (Variables|Default|GetCounter))))
    (:Completed
      (if (== (Utilities|Array|LastIndex _light) (Variables|Default|GetCounter))
        (CallFunction|Open)
        (else
          (CallFunction|Close))))))

(fn OpenDoor
  (CallFunction|Open))

(fn LoadNewLevel
  (Game|OpenLevel(byObjectReference) (Variables|Default|GetLevel)))