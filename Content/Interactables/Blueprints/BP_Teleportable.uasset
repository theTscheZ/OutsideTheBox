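; BP_Teleportable is an interactable object with a static mesh that can be resized and reports a weight.
; It caches the mesh's world scale on BeginPlay as the default.
; The Resize event scales the mesh relative to that default and sets Weight to the same multiplier, which GetWeight returns.
; The file itself contains no teleport logic.
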(event Custom|Resize
  (params (Multiplier :type Float%20%28double-precision%29))
  (bind _output_get (Variables|Default|SetMultiplier Multiplier))
  (Variables|Default|SetWeight _output_get)
  (Transformation|SetWorldScale3D (Variables|Default|GetStaticMesh) (* (Variables|Default|GetDefaultScale) _output_get)))

(event EventBeginPlay
  (Variables|Default|SetDefaultScale (Transformation|GetWorldScale (Variables|Default|GetStaticMesh))))

(event Collision|EventActorBeginOverlap
  (params (OtherActor :type Actor%20Object%20Reference)))

(event EventTick
  (params (DeltaSeconds :type Float%20%28single-precision%29)))

(fn ConstructionScript)

(fn GetWeight
  (return (Variables|Default|GetWeight)))