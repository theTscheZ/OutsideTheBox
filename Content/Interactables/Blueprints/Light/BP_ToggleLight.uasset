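; BP_ToggleLight is a lamp that shows an on or off state through its glow and reports to a linked gate.
; The construction script creates a dynamic instance of the glowing material and sets its emissive multiplier from IsLightOn.
; SetLight asks the gate assigned through SetGate to check the lights, then refreshes the glow to match the current flag, which this Blueprint never changes itself.
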(event EventBeginPlay)

(event Collision|EventActorBeginOverlap
  (params (OtherActor :type Actor%20Object%20Reference)))

(event EventTick
  (params (DeltaSeconds :type Float%20%28single-precision%29)))

(fn ConstructionScript
  (bind _returnvalue (Rendering|Material|CreateDynamicMaterialInstance (Variables|Default|GetLamp) 0 "/Game/Interactables/Blueprints/Light/Glowing_MAT.Glowing_MAT" "None" :!class /Script/Engine.PrimitiveComponent))
  (Variables|Default|SetLampMaterial _returnvalue)
  (if (Variables|Default|GetIsLightOn?)
    (Rendering|Material|SetScalarParameterValue (Variables|Default|GetLampMaterial) "EmissiveMultiplier" 1.0 :!class /Script/Engine.MaterialInstanceDynamic)
    (else
      (Rendering|Material|SetScalarParameterValue (Variables|Default|GetLampMaterial) "EmissiveMultiplier" 0.0 :!class /Script/Engine.MaterialInstanceDynamic))))

(fn SetGate
  (params (set%20Gate :type BP%20Gate%20Object%20Reference))
  (Variables|Default|SetGate set%20Gate))

(fn SetLight
  (bind _lampmaterial (Variables|Default|GetLampMaterial))
  (bind _gate (Variables|Default|GetGate))
  (Utilities|IsValid _gate
    (:Is%20Valid
      (Default|CheckLight _gate))
    (:Is%20Not%20Valid
      _))
  (if (Variables|Default|GetIsLightOn?)
    (Rendering|Material|SetScalarParameterValue _lampmaterial "EmissiveMultiplier" 1.0 :!class /Script/Engine.MaterialInstanceDynamic)
    (else
      (Rendering|Material|SetScalarParameterValue _lampmaterial "EmissiveMultiplier" 0.0 :!class /Script/Engine.MaterialInstanceDynamic))))