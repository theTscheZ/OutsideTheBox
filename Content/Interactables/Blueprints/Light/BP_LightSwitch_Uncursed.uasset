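; An interactable light switch Blueprint that toggles a set of linked lamps.
; Interact flips the switch state and plays or reverses a Timeline that pitches the lever shaft.
; When the Timeline finishes in either direction, each lamp in the Lamps array has its IsLightOn flag inverted and SetLight called, so lamps toggle individually rather than copy the switch state.
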(event EventBeginPlay)

(event Collision|EventActorBeginOverlap
  (params (OtherActor :type Actor%20Object%20Reference)))

(event EventTick
  (params (DeltaSeconds :type Float%20%28single-precision%29)))

(event EventInteract
  (params (Interacting%20Player :type BP%20First%20Person%20Character%20Object%20Reference))
  (if (Variables|Default|GetSwitch_On?)
    (Variables|Default|SetSwitch_On? false)
    (bind _cursed_as_hell_y_axis (Timeline|Switch_Animation Reverse)
      (:Update
        (Transformation|SetRelativeRotation (Variables|Default|GetLever_Shaft) (Math|Rotator|MakeRotator 0.0 _cursed_as_hell_y_axis 0.0) false false))
      (:Finished
        (for _array_element (Variables|Default|GetLamps)
          (if (Variables|/Game/Interactables/Blueprints/Light/BP_ToggleLight.BP_ToggleLight_C|GetIsLightOn? _array_element)
            (Variables|/Game/Interactables/Blueprints/Light/BP_ToggleLight.BP_ToggleLight_C|SetIsLightOn? _array_element false)
            (else
              (Variables|/Game/Interactables/Blueprints/Light/BP_ToggleLight.BP_ToggleLight_C|SetIsLightOn? _array_element true)))
          (Default|SetLight _array_element))))
    (else
      (Variables|Default|SetSwitch_On? true)
      (Timeline|Switch_Animation Play))))

(fn ConstructionScript)