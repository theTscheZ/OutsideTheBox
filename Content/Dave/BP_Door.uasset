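; BP_Door is a door actor that opens while enough pressure switches are active.
; SwitchActivated and SwitchDeactivated adjust a counter of active switches and compare it to the required count.
; Meeting the count plays the DoorOpening timeline and falling short reverses it, with the timeline driving the door's relative Z location.
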(event Custom|SwitchActivated
  (bind _result (Math|Integer|IncrementInt (Variables|Default|GetPressureSwitchesActive))
    (:%20%20
      (if (>= _result (Variables|Default|GetPressureSwitchesNeeded))
        (bind _doorposition (Timeline|DoorOpening Play)
          (:Update
            (Transformation|SetRelativeLocation (Variables|Default|GetDoor) (Math|Vector|MakeVector 0.0 0.0 _doorposition) false false)))
        (else
          (Timeline|DoorOpening Reverse))))))

(event Custom|SwitchDeactivated
  (bind _result (Math|Integer|DecrementInt (Variables|Default|GetPressureSwitchesActive))
    (:%20%20
      (if (>= _result (Variables|Default|GetPressureSwitchesNeeded))
        (bind _doorposition (Timeline|DoorOpening Play)
          (:Update
            (Transformation|SetRelativeLocation (Variables|Default|GetDoor) (Math|Vector|MakeVector 0.0 0.0 _doorposition) false false)))
        (else
          (Timeline|DoorOpening Reverse))))))

(event EventBeginPlay)

(event Collision|EventActorBeginOverlap
  (params (OtherActor :type Actor%20Object%20Reference)))

(event EventTick
  (params (DeltaSeconds :type Float%20%28single-precision%29)))

(fn ConstructionScript)