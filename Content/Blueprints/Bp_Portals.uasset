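; Linked portal actor that shows the view through its partner and teleports the player and BPI_Teleportable objects to it.
; The partner's scene capture mirrors the player camera each post-update tick, feeding a viewport-sized render target on the portal material, with clip planes.
; While enabled, overlapping actors teleport when a velocity-predicted dot-product test detects crossing.
; Teleports remap rotation to the exit, but only the player's velocity is carried over.
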(event OnComponentBeginOverlap(Teleport)
  (params (OverlappedComponent :type Primitive%20Component%20Object%20Reference) (OtherActor :type Actor%20Object%20Reference) (OtherComp :type Primitive%20Component%20Object%20Reference) (OtherBodyIndex :type Integer) (bFromSweep :type Boolean) (SweepResult :type Hit%20Result%20Structure%20%28by%20ref%29))
  (Utilities|Casting|CastToBP_FirstPersonCharacter OtherActor
    (:then
      (Variables|Default|SetisPlayerOverlap true))
    (:CastFailed
      (if (Utilities|DoesObjectImplementInterface OtherActor "/Game/Interfaces/BPI_Teleportable.BPI_Teleportable_C")
        (Variables|Default|SetStartOverlap true)
        (Variables|Default|SetObject OtherActor)))))

(event OnComponentEndOverlap(Teleport)
  (params (OverlappedComponent :type Primitive%20Component%20Object%20Reference) (OtherActor :type Actor%20Object%20Reference) (OtherComp :type Primitive%20Component%20Object%20Reference) (OtherBodyIndex :type Integer))
  (Utilities|Casting|CastToBP_FirstPersonCharacter OtherActor
    (:then
      (Variables|Default|SetisPlayerOverlap false))
    (:CastFailed
      (if (Utilities|DoesObjectImplementInterface OtherActor "/Game/Interfaces/BPI_Teleportable.BPI_Teleportable_C")
        (Variables|Default|SetStartOverlap false)
        (Variables|Default|SetObject 0)))))

(event EventBeginPlay
  (bind _returnvalue (Viewport|GetViewportSize))
  (bind _arrow (Variables|Default|GetArrow))
  (bind _offset_rotation (Variables|Default|GetOffset%20rotation))
  (bind _returnvalue_2 (Math|Vector|GetForwardVector _arrow))
  (bind _returnvalue_3 (* _returnvalue_2 _offset_rotation))
  (bind (_x _y _z) (Math|Vector|BreakVector _returnvalue_3))
  (bind _asbp_first_person_character (Utilities|Casting|CastToBP_FirstPersonCharacter (Game|GetPlayerCharacter 0)))
  (Variables|Default|SetAs%20BP%20First%20Person%20Character _asbp_first_person_character)
  (Components|Tick|SetTickGroup "TG_PostUpdateWork")
  (bind _returnvalue_4 (Rendering|Material|CreateDynamicMaterialInstance "/Game/Blueprints/NewFolder/Portal.Portal" "None" "None" :!class /Script/Engine.KismetMaterialLibrary))
  (bind _output_get (Variables|Default|SetPortal%20_mat _returnvalue_4))
  (Rendering|Material|SetMaterial (Variables|Default|GetPlane) 0 _output_get)
  (bind _returnvalue_5 (Rendering|CreateRenderTarget2D (Math|Float|Truncate (.x _returnvalue)) (Math|Float|Truncate (.y _returnvalue)) "RTF_RGBA16f"))
  (bind _output_get_2 (Variables|Default|SetPortal_RT _returnvalue_5))
  ;[1 1 1] bei gott wehe einer von euch änder den namen
  (Rendering|Material|SetTextureParameterValue (Variables|Default|GetPortal%20_mat) "Texture" _output_get_2)
  (Variables|/Script/Engine.SceneCaptureComponent2D|SetTextureTarget (Variables|Bp_Portals_C|GetSceneCaptureComponent2D (Variables|Default|GetLinkedPortal)) (Variables|Default|GetPortal_RT))
  (CallFunction|SetClipping)
  (Rendering|Material|SetVectorParameterValue (Variables|Default|GetPortal%20_mat) "OffsetDistance" (Math|Color|MakeColor _x _y _z) :!class /Script/Engine.MaterialInstanceDynamic))

(event Collision|EventActorBeginOverlap
  (params (OtherActor :type Actor%20Object%20Reference)))

(event EventTick
  (params (DeltaSeconds :type Float%20%28single-precision%29))
  (CallFunction|UpdateScene)
  (CallFunction|CheckViewportSize)
  (if (Variables|Default|GetIsEnabled)
    (if (Variables|Default|GetisPlayerOverlap)
      (CallFunction|UpdateRenderTargetPlayer)
      (else
        (CallFunction|UpdateRenderTargetObject)))))

(fn ConstructionScript)

(fn UpdateRenderTargetPlayer
  (bind _returnvalue (Viewport|GetViewportSize))
  (bind _teleportationpoint4player (Variables|Default|GetTeleportationPoint4Player))
  (bind _as_bp_first_person_character (Variables|Default|GetAs%20BP%20First%20Person%20Character))
  (bind _scenecapturecomponent2d (Variables|Default|GetSceneCaptureComponent2D))
  (Rendering|ResizeRenderTarget2D (Variables|/Script/Engine.SceneCaptureComponent2D|GetTextureTarget (Variables|Default|GetSceneCaptureComponent2D)) (Math|Float|Truncate (.x _returnvalue)) (Math|Float|Truncate (.y _returnvalue)))
  (bind _as_bp_first_person_character_2 (Variables|Default|GetAs%20BP%20First%20Person%20Character)
    (:then
      (Transformation|SetRelativeLocationAndRotation (Variables|Bp_Portals_C|GetSceneCaptureComponent2D (Variables|Default|GetLinkedPortal)) (.location (Math|Transform|MakeRelativeTransform (Transformation|GetWorldTransform (Variables|/Game/FirstPerson/Blueprints/BP_FirstPersonCharacter.BP_FirstPersonCharacter_C|GetFirstPersonCamera _as_bp_first_person_character_2)) (Transformation|GetWorldTransform (Variables|Default|GetBackfacing)))) "0, 0, 0" false false)
      ;[0.01042 0.01042 0.01042] Clipping mask
      (Variables|/Script/Engine.SceneCaptureComponent2D|SetClipPlaneBase _scenecapturecomponent2d (Transformation|GetWorldLocation (Variables|Default|GetPlane)))
      (Variables|/Script/Engine.SceneCaptureComponent2D|SetClipPlaneNormal _scenecapturecomponent2d (Math|Vector|GetForwardVector (Variables|Default|GetArrow)))
      (if (Variables|Default|GetisPlayerOverlap)
        (if (>= (Math|Vector|DotProduct (Math|Vector|GetForwardVector _teleportationpoint4player) (Math|Vector|Normalize (- (Transformation|GetWorldLocation _teleportationpoint4player) (+ (Transformation|GetActorLocation _as_bp_first_person_character) (* (+ (Transformation|GetVelocity _as_bp_first_person_character) "2.000000,0.000000,0.000000") (Utilities|Time|GetWorldDeltaSeconds)))))) 0.0)
          (CallFunction|PlayerTeleport))))
    (:else)))

(fn PlayerTeleport
  (bind _as_bp_first_person_character (Variables|Default|GetAs%20BP%20First%20Person%20Character))
  (bind _teleportationpoint4player (Variables|Default|GetTeleportationPoint4Player))
  (bind _linkedportal (Variables|Default|GetLinkedPortal))
  (bind _returnvalue (Transformation|GetWorldTransform _teleportationpoint4player))
  (bind _returnvalue_2 (Pawn|GetController _as_bp_first_person_character))
  (bind _backfacing (Variables|Bp_Portals_C|GetBackfacing _linkedportal))
  (bind _returnvalue_3 (Pawn|GetControlRotation _returnvalue_2 :!class /Script/Engine.Controller))
  (bind _returnvalue_4 (Transformation|GetWorldTransform _backfacing))
  (bind _returnvalue_5 (Math|Transform|InverseTransformRotation _returnvalue _returnvalue_3))
  (bind _returnvalue_6 (Math|Transform|TransformRotation _returnvalue_4 _returnvalue_5))
  (Development|PrintString (Utilities|String|ToString(Vector) (Transformation|GetActorLocation (Variables|Default|GetAs%20BP%20First%20Person%20Character))))
  (LocalVariables|SetL-Velocity (Math|Transform|TransformDirection (Transformation|GetWorldTransform (Variables|Bp_Portals_C|GetBackfacing (Variables|Default|GetLinkedPortal))) (Math|Transform|InverseTransformDirection (Transformation|GetWorldTransform (Variables|Default|GetTeleportationPoint4Player)) (Transformation|GetVelocity (Variables|Default|GetAs%20BP%20First%20Person%20Character)))))
  (LocalVariables|SetL-Position (Math|Transform|TransformLocation (Transformation|GetWorldTransform (Variables|Bp_Portals_C|GetBackfacing (Variables|Default|GetLinkedPortal))) "0, 0, 0"))
  (LocalVariables|SetL-Rotation (Math|Rotator|MakeRotator 0.0 (.pitch _returnvalue_6) (.yaw _returnvalue_6)))
  (Pawn|SetControlRotation (Pawn|GetController (Variables|Default|GetAs%20BP%20First%20Person%20Character)) (LocalVariables|GetL-Rotation))
  (Transformation|SetActorLocationAndRotation (Variables|Default|GetAs%20BP%20First%20Person%20Character) (LocalVariables|GetL-Position) (LocalVariables|GetL-Rotation))
  (Variables|/Script/Engine.MovementComponent|SetVelocity (Variables|/Script/Engine.Character|GetCharacterMovement (Variables|Default|GetAs%20BP%20First%20Person%20Character)) (LocalVariables|GetL-Velocity))
  (if (Variables|Default|GetisSize)
    _))

(fn ObjectTeleport
  (bind _linkedportal (Variables|Default|GetLinkedPortal))
  (bind _object (Variables|Default|GetObject))
  (bind _teleportationpoint4player (Variables|Default|GetTeleportationPoint4Player))
  (bind _returnvalue (Transformation|GetWorldTransform _teleportationpoint4player))
  (bind _returnvalue_2 (Transformation|GetActorRotation _object))
  (bind _backfacing (Variables|Bp_Portals_C|GetBackfacing _linkedportal))
  (bind _returnvalue_3 (Math|Transform|InverseTransformRotation _returnvalue _returnvalue_2))
  (bind _returnvalue_4 (Transformation|GetWorldTransform _backfacing))
  (bind _returnvalue_5 (Math|Transform|TransformRotation _returnvalue_4 _returnvalue_3))
  (Development|PrintString (Utilities|String|ToString(Vector) (Transformation|GetActorLocation (Variables|Default|GetObject))))
  (LocalVariables|SetL-Velocity (Math|Transform|TransformDirection (Transformation|GetWorldTransform (Variables|Bp_Portals_C|GetBackfacing (Variables|Default|GetLinkedPortal))) (Math|Transform|InverseTransformDirection (Transformation|GetWorldTransform (Variables|Default|GetTeleportationPoint4Player)) (Transformation|GetVelocity (Variables|Default|GetObject)))))
  (LocalVariables|SetL-Position (Math|Transform|TransformLocation (Transformation|GetWorldTransform (Variables|Bp_Portals_C|GetBackfacing (Variables|Default|GetLinkedPortal))) "0, 0, 0"))
  (bind _output_get (LocalVariables|SetL-Rotation (Math|Rotator|MakeRotator 0.0 (.pitch _returnvalue_5) (.yaw _returnvalue_5))))
  (Transformation|SetActorLocationAndRotation (Variables|Default|GetObject) (LocalVariables|GetL-Position) _output_get)
  (if (Variables|Default|GetisSize)
    _))

(fn UpdateRenderTargetObject
  (bind _teleportationpoint4object (Variables|Default|GetTeleportationPoint4Object))
  (bind _object (Variables|Default|GetObject))
  (if (Variables|Default|GetStartOverlap)
    (if (>= (Math|Vector|DotProduct (Math|Vector|GetForwardVector _teleportationpoint4object) (Math|Vector|Normalize (- (Transformation|GetWorldLocation _teleportationpoint4object) (+ (Transformation|GetActorLocation _object) (* (Transformation|GetVelocity _object) (Utilities|Time|GetWorldDeltaSeconds)))))) 0.0)
      (CallFunction|ObjectTeleport))))

(fn UpdateScene
  (bind _returnvalue (Transformation|GetActorTransform))
  (bind _returnvalue_2 (Game|GetPlayerCameraManager 0))
  (bind _returnvalue_3 (Transformation|GetActorTransform))
  (bind _linkedportal (Variables|Default|GetLinkedPortal))
  (bind (_location _rotation _scale) (Math|Transform|BreakTransform _returnvalue))
  (bind _returnvalue_4 (Transformation|GetActorTransform _linkedportal))
  (bind _transformcomponent (Variables|/Script/Engine.PlayerCameraManager|GetTransformComponent _returnvalue_2))
  (bind (_x _y _z) (Math|Vector|BreakVector _scale))
  (bind _returnvalue_5 (Transformation|GetWorldRotation _transformcomponent))
  (bind (_x_2 _y_2 _z_2) (Math|Rotator|BreakRotIntoAxes _returnvalue_5))
  (Transformation|SetWorldLocationAndRotation (Variables|Bp_Portals_C|GetSceneCaptureComponent2D (Variables|Default|GetLinkedPortal)) (Math|Transform|TransformLocation (Transformation|GetActorTransform (Variables|Default|GetLinkedPortal)) (Math|Transform|InverseTransformLocation (Math|Transform|MakeTransform _location _rotation (Math|Vector|MakeVector (* _x -1.0) (* _y -1.0) _z)) (Transformation|GetWorldLocation (Variables|/Script/Engine.PlayerCameraManager|GetTransformComponent (Game|GetPlayerCameraManager 0))))) (Math|Rotator|MakeRotationfromAxes (Math|Transform|TransformDirection _returnvalue_4 (Math|Vector|MirrorVectorbyNormal (Math|Vector|MirrorVectorbyNormal (Math|Transform|InverseTransformDirection _returnvalue_3 _x_2) "-1.000000,0.000000,0.000000") "0.000000,2.000000,0.000000")) (Math|Transform|TransformDirection _returnvalue_4 (Math|Vector|MirrorVectorbyNormal (Math|Vector|MirrorVectorbyNormal (Math|Transform|InverseTransformDirection _returnvalue_3 _y_2) "-1.000000,0.000000,0.000000") "0.000000,2.000000,0.000000")) (Math|Transform|TransformDirection _returnvalue_4 (Math|Vector|MirrorVectorbyNormal (Math|Vector|MirrorVectorbyNormal (Math|Transform|InverseTransformDirection _returnvalue_3 _z_2) "-1.000000,0.000000,0.000000") "0.000000,2.000000,0.000000"))) false false))

(fn SetClipping
  (bind _scenecapturecomponent2d (Variables|Default|GetSceneCaptureComponent2D))
  (Utilities|IsValid (Variables|Default|GetLinkedPortal)
    (:Is%20Valid
      (Variables|/Script/Engine.SceneCaptureComponent2D|SetbEnableClipPlane _scenecapturecomponent2d true)
      (Variables|/Script/Engine.SceneCaptureComponent2D|SetClipPlaneBase _scenecapturecomponent2d (+ (Transformation|GetWorldLocation (Variables|Default|GetPlane)) (+ (Math|Vector|GetForwardVector (Variables|Default|GetArrow)) -3.0)))
      (Variables|/Script/Engine.SceneCaptureComponent2D|SetClipPlaneNormal _scenecapturecomponent2d (Math|Vector|GetForwardVector (Variables|Default|GetArrow))))))

(fn CheckViewportSize
  (bind _returnvalue (Viewport|GetViewportSize))
  (bind _returnvalue_2 (Viewport|GetViewportSize))
  (bind _portal_rt (Variables|Default|GetPortal_RT))
  (bind (_x _y) (Math|Vector2D|BreakVector2D _returnvalue))
  (bind (_x_2 _y_2) (Math|Vector2D|BreakVector2D _returnvalue_2))
  (if (not (and (== _x (Variables|/Script/Engine.TextureRenderTarget2D|GetSizeX _portal_rt)) (== _y (Variables|/Script/Engine.TextureRenderTarget2D|GetSizeY _portal_rt))))
    (Rendering|ResizeRenderTarget2D (Variables|Default|GetPortal_RT) (Math|Float|Truncate _x_2) (Math|Float|Truncate _y_2))))