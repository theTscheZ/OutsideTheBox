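; Linked portal actor that shows a see-through view of its partner and teleports the first-person player across.
; Each tick after update work, the partner's clip-planed scene capture renders the mirrored player view into a viewport-sized render target on this portal's material.
; Recursion up to MaxR captures deepest first, producing nested portal views.
; When the camera crosses the portal plane front-to-back, player transform, control rotation and velocity are remapped to the partner.
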(event EventBeginPlay
  (bind _returnvalue (Viewport|GetViewportSize))
  (bind _arrow (Variables|Default|GetArrow))
  (bind _offset (Variables|Default|GetOffset))
  (bind _returnvalue_2 (Math|Vector|GetForwardVector _arrow))
  (bind _returnvalue_3 (* _returnvalue_2 _offset))
  (bind (_x _y _z) (Math|Vector|BreakVector _returnvalue_3))
  (Components|Tick|SetTickGroup "TG_PostUpdateWork")
  (bind _returnvalue_4 (Rendering|Material|CreateDynamicMaterialInstance "/Game/Blueprints/portal/Portal_uwu_MA.Portal_uwu_MA" "None" "None" :!class /Script/Engine.KismetMaterialLibrary))
  (bind _output_get (Variables|Default|SetPortal_Mat _returnvalue_4))
  (Rendering|Material|SetMaterial (Variables|Default|GetPortal) 0 _output_get)
  (bind _returnvalue_5 (Rendering|CreateRenderTarget2D (Math|Float|Truncate (.x _returnvalue)) (Math|Float|Truncate (.y _returnvalue)) "RTF_RGBA16f"))
  (bind _output_get_2 (Variables|Default|SetPortal_RT _returnvalue_5))
  (Rendering|Material|SetTextureParameterValue (Variables|Default|GetPortal_Mat) "Texture" _output_get_2)
  (Variables|/Script/Engine.SceneCaptureComponent2D|SetTextureTarget (Variables|UwU_Portal_C|GetPortalCamera (Variables|Default|GetLinked%20Portal)) (Variables|Default|GetPortal_RT))
  (CallFunction|SetClipPlanes)
  (Rendering|Material|SetVectorParameterValue (Variables|Default|GetPortal_Mat) "OffsetDistance" (Math|Color|MakeColor _x _y _z) :!class /Script/Engine.MaterialInstanceDynamic))

(event Collision|EventActorBeginOverlap
  (params (OtherActor :type Actor%20Object%20Reference)))

(event EventTick
  (params (DeltaSeconds :type Float%20%28single-precision%29))
  (CallFunction|UpdateScenecaptureRecusive# "0, 0, 0" "0, 0, 0")
  (CallFunction|CheckViewportSize)
  (CallFunction|ShouldTeleport))

(fn ConstructionScript)

(fn UpdateSceneCapture
  (Transformation|SetWorldLocationAndRotation (Variables|UwU_Portal_C|GetPortalCamera (Variables|Default|GetLinked%20Portal)) (CallFunction|UpdateLocation "0, 0, 0") (CallFunction|UpdateRoataion "0, 0, 0") false false))

(fn SetClipPlanes
  (bind _portalcamera (Variables|Default|GetPortalCamera))
  (Utilities|IsValid (Variables|Default|GetLinked%20Portal)
    (:Is%20Valid
      (Variables|/Script/Engine.SceneCaptureComponent2D|SetbEnableClipPlane _portalcamera true)
      (Variables|/Script/Engine.SceneCaptureComponent2D|SetClipPlaneBase _portalcamera (+ (Transformation|GetWorldLocation (Variables|Default|GetPortal)) (* (Math|Vector|GetForwardVector (Variables|Default|GetArrow)) -3.0)))
      (Variables|/Script/Engine.SceneCaptureComponent2D|SetClipPlaneNormal _portalcamera (Math|Vector|GetForwardVector (Variables|Default|GetArrow))))))

(fn CheckViewportSize
  (bind _returnvalue (Viewport|GetViewportSize))
  (bind _returnvalue_2 (Viewport|GetViewportSize))
  (bind _portal_rt (Variables|Default|GetPortal_RT))
  (bind (_x _y) (Math|Vector2D|BreakVector2D _returnvalue))
  (if (not (and (== _x (Variables|/Script/Engine.TextureRenderTarget2D|GetSizeX _portal_rt)) (== _y (Variables|/Script/Engine.TextureRenderTarget2D|GetSizeY _portal_rt))))
    (Development|PrintString "Hello")
    (Rendering|ResizeRenderTarget2D (Variables|Default|GetPortal_RT) (Math|Float|Truncate (.x _returnvalue_2)) (Math|Float|Truncate (.y _returnvalue_2)))))

(fn ShouldTeleport
  (Utilities|IsValid (Utilities|Array|Get(acopy) (Collision|GetOverlappingActors (Variables|Default|GetPlayer%20Detection) "/Game/FirstPerson/Blueprints/BP_FirstPersonCharacter.BP_FirstPersonCharacter_C" :!class /Script/Engine.PrimitiveComponent))
    (:Is%20Valid
      (bind _retrun (CallFunction|IsPointCrossingPortal? (Transformation|GetWorldLocation (Variables|/Game/FirstPerson/Blueprints/BP_FirstPersonCharacter.BP_FirstPersonCharacter_C|GetFirstPersonCamera (.AsBP%20First%20Person%20Character (Utilities|Casting|CastToBP_FirstPersonCharacter (Game|GetPlayerCharacter 0))))) (Transformation|GetActorLocation) (Math|Vector|GetForwardVector (Variables|Default|GetArrow))))
      (if _retrun
        (CallFunction|TeleportCharacter)))))

(fn IsPointCrossingPortal?
  (params (point :type Vector) (PortalLocation :type Vector) (PortalNormal :type Vector))
  (LocalVariables|SetIsInFront (>= (Math|Vector|DotProduct PortalNormal (- point PortalLocation)) 0.0))
  (bind _output_get (LocalVariables|SetPortalPlane (Class|KismetMathLibrary|MakePlanefromPointandNormal PortalLocation PortalNormal)))
  (LocalVariables|SetIsIntersect (.ReturnValue (Class|KismetMathLibrary|LinePlaneIntersection (Variables|Default|GetLastPosition) point _output_get)))
  (LocalVariables|SetIsCrossing (Math|Boolean|ANDBoolean (LocalVariables|GetIsIntersect) (not (LocalVariables|GetIsInFront)) (Variables|Default|GetLastInFront)))
  (Variables|Default|SetLastInFront (LocalVariables|GetIsInFront))
  (Variables|Default|SetLastPosition point)
  (return (LocalVariables|GetIsCrossing)))

(fn TeleportCharacter
  (bind _returnvalue (Transformation|GetActorTransform))
  (bind _returnvalue_2 (Game|GetPlayerCharacter 0))
  (bind _returnvalue_3 (Transformation|GetActorTransform))
  (bind _returnvalue_4 (Transformation|GetActorTransform))
  (bind _returnvalue_5 (Game|GetPlayerCharacter 0))
  (bind _returnvalue_6 (Game|GetPlayerController 0))
  (bind _linked_portal (Variables|Default|GetLinked%20Portal))
  (bind _linked_portal_2 (Variables|Default|GetLinked%20Portal))
  (bind _linked_portal_3 (Variables|Default|GetLinked%20Portal))
  (bind _returnvalue_7 (Pawn|GetMovementComponent _returnvalue_2))
  (bind _returnvalue_8 (Transformation|GetActorTransform _linked_portal))
  (bind _returnvalue_9 (Transformation|GetActorTransform _linked_portal_2))
  (bind _returnvalue_10 (Transformation|GetActorTransform _linked_portal_3))
  (bind _returnvalue_11 (Transformation|GetActorRotation _returnvalue_5))
  (bind _returnvalue_12 (Pawn|GetControlRotation _returnvalue_6 :!class /Script/Engine.Controller))
  (bind (_x _y _z) (Math|Vector|BreakVector (.scale _returnvalue)))
  (bind (_x_2 _y_2 _z_2) (Math|Rotator|GetAxes _returnvalue_12))
  (bind (_x_3 _y_3 _z_3) (Math|Rotator|GetAxes _returnvalue_11))
  (bind _returnvalue_13 (Math|Transform|InverseTransformDirection _returnvalue_3 _z_2))
  (bind _returnvalue_14 (Math|Transform|InverseTransformDirection _returnvalue_3 _x_2))
  (bind _returnvalue_15 (Math|Transform|InverseTransformDirection _returnvalue_3 _y_2))
  (bind _returnvalue_16 (Math|Vector|MirrorVectorbyNormal _returnvalue_13 "1.000000,0.000000,0.000000"))
  (bind _returnvalue_17 (Math|Vector|MirrorVectorbyNormal _returnvalue_14 "1.000000,0.000000,0.000000"))
  (bind _returnvalue_18 (Math|Vector|MirrorVectorbyNormal _returnvalue_15 "1.000000,0.000000,0.000000"))
  (bind _returnvalue_19 (Math|Vector|MirrorVectorbyNormal _returnvalue_16 "0.000000,1.000000,0.000000"))
  (bind _returnvalue_20 (Math|Vector|MirrorVectorbyNormal _returnvalue_17 "0.000000,1.000000,0.000000"))
  (bind _returnvalue_21 (Math|Vector|MirrorVectorbyNormal _returnvalue_18 "0.000000,1.000000,0.000000"))
  (bind _returnvalue_22 (Math|Transform|TransformDirection _returnvalue_8 _returnvalue_19))
  (bind _returnvalue_23 (Math|Transform|TransformDirection _returnvalue_9 _returnvalue_20))
  (bind _returnvalue_24 (Math|Transform|TransformDirection _returnvalue_10 _returnvalue_21))
  (bind _returnvalue_25 (Math|Rotator|MakeRotationfromAxes _returnvalue_23 _returnvalue_24 _returnvalue_22))
  (Transformation|SetActorTransform (Game|GetPlayerCharacter 0) (Math|Transform|MakeTransform (Math|Transform|TransformLocation (Transformation|GetActorTransform (Variables|Default|GetLinked%20Portal)) (Math|Transform|InverseTransformLocation (Math|Transform|MakeTransform (.location _returnvalue) (.rotation _returnvalue) (Math|Vector|MakeVector (* _x -1.0) (* _y -1.0) _z)) (Transformation|GetActorLocation (Game|GetPlayerCharacter 0)))) (Math|Rotator|MakeRotationfromAxes (Math|Transform|TransformDirection (Transformation|GetActorTransform (Variables|Default|GetLinked%20Portal)) (Math|Vector|MirrorVectorbyNormal (Math|Vector|MirrorVectorbyNormal (Math|Transform|InverseTransformDirection _returnvalue_4 _x_3) "1.000000,0.000000,0.000000") "0.000000,1.000000,0.000000")) (Math|Transform|TransformDirection (Transformation|GetActorTransform (Variables|Default|GetLinked%20Portal)) (Math|Vector|MirrorVectorbyNormal (Math|Vector|MirrorVectorbyNormal (Math|Transform|InverseTransformDirection _returnvalue_4 _y_3) "1.000000,0.000000,0.000000") "0.000000,1.000000,0.000000")) (Math|Transform|TransformDirection (Transformation|GetActorTransform (Variables|Default|GetLinked%20Portal)) (Math|Vector|MirrorVectorbyNormal (Math|Vector|MirrorVectorbyNormal (Math|Transform|InverseTransformDirection _returnvalue_4 _z_3) "1.000000,0.000000,0.000000") "0.000000,1.000000,0.000000"))) "1.000000,1.000000,1.000000"))
  (Pawn|SetControlRotation (Game|GetPlayerController 0) _returnvalue_25)
  (bind _retrun_value (CallFunction|UpdateVelocity (Variables|/Script/Engine.MovementComponent|GetVelocity _returnvalue_7)))
  (Variables|/Script/Engine.MovementComponent|SetVelocity _returnvalue_7 _retrun_value)
  (Default|SmoothOrientation (.AsBP%20First%20Person%20Character (Utilities|Casting|CastToBP_FirstPersonCharacter (Game|GetPlayerCharacter 0))) _returnvalue_25)
  (Class|PlayerCameraManager|SetGameCameraCutThisFrame (Game|GetPlayerCameraManager 0)))

(fn UpdateVelocity
  (params (Velocity :type Vector))
  (return (* (Math|Transform|TransformDirection (Transformation|GetActorTransform (Variables|Default|GetLinked%20Portal)) (Math|Vector|MirrorVectorbyNormal (Math|Vector|MirrorVectorbyNormal (Math|Transform|InverseTransformDirection (Transformation|GetActorTransform) (Math|Vector|Normalize Velocity)) "1.000000,0.000000,0.000000") "0.000000,1.000000,0.000000")) (* (Transformation|GetVelocity) "1.500000,1.500000,1.500000"))))

(fn UpdateLocation
  (params (Old%20Location :type Vector))
  (bind _returnvalue (Transformation|GetActorTransform))
  (bind (_location _rotation _scale) (Math|Transform|BreakTransform _returnvalue))
  (bind (_x _y _z) (Math|Vector|BreakVector _scale))
  (return (Math|Transform|TransformLocation (Transformation|GetActorTransform (Variables|Default|GetLinked%20Portal)) (Math|Transform|InverseTransformLocation (Math|Transform|MakeTransform _location _rotation (Math|Vector|MakeVector (* _x -1.0) (* _y -1.0) _z)) Old%20Location))))

(fn UpdateRoataion
  (params (OldRotation :type Rotator))
  (bind (_x _y _z) (Math|Rotator|BreakRotIntoAxes OldRotation))
  (bind _returnvalue (Transformation|GetActorTransform))
  (bind _linked_portal (Variables|Default|GetLinked%20Portal))
  (bind _returnvalue_2 (Transformation|GetActorTransform _linked_portal))
  (return (Math|Rotator|MakeRotationfromAxes (Math|Transform|TransformDirection _returnvalue_2 (Math|Vector|MirrorVectorbyNormal (Math|Vector|MirrorVectorbyNormal (Math|Transform|InverseTransformDirection _returnvalue _x) "1.000000,0.000000,0.000000") "0.000000,1.000000,0.000000")) (Math|Transform|TransformDirection _returnvalue_2 (Math|Vector|MirrorVectorbyNormal (Math|Vector|MirrorVectorbyNormal (Math|Transform|InverseTransformDirection _returnvalue _y) "1.000000,0.000000,0.000000") "0.000000,1.000000,0.000000")) (Math|Transform|TransformDirection _returnvalue_2 (Math|Vector|MirrorVectorbyNormal (Math|Vector|MirrorVectorbyNormal (Math|Transform|InverseTransformDirection _returnvalue _z) "1.000000,0.000000,0.000000") "0.000000,1.000000,0.000000")))))

(fn UpdateScenecaptureRecusive#
  (params (location :type Vector) (Rotation :type Rotator))
  (bind _returnvalue (Game|GetPlayerCameraManager 0))
  (bind _transformcomponent (Variables|/Script/Engine.PlayerCameraManager|GetTransformComponent _returnvalue))
  (if (== (Variables|Default|GetCurrentRecursion) 0)
    (LocalVariables|SetTemporaryLocation (CallFunction|UpdateLocation (Transformation|GetWorldLocation _transformcomponent)))
    (LocalVariables|Settemp%20rotation (CallFunction|UpdateRoataion (Transformation|GetWorldRotation _transformcomponent)))
    (Math|Integer|IncrementInt (Variables|Default|GetCurrentRecursion)
      (:%20%20
        (CallFunction|UpdateScenecaptureRecusive# (LocalVariables|GetTemporaryLocation) (LocalVariables|Gettemp%20rotation))
        (Transformation|SetWorldLocationAndRotation (Variables|UwU_Portal_C|GetPortalCamera (Variables|Default|GetLinked%20Portal)) (LocalVariables|GetTemporaryLocation) (LocalVariables|Gettemp%20rotation) false false)
        (Rendering|SceneCapture|CaptureScene (Variables|UwU_Portal_C|GetPortalCamera (Variables|Default|GetLinked%20Portal)) :!class /Script/Engine.SceneCaptureComponent2D)
        (Variables|Default|SetCurrentRecursion 0)))
    (elif (< (Variables|Default|GetCurrentRecursion) (Variables|Default|GetMaxR))
      (LocalVariables|SetTemporaryLocation (CallFunction|UpdateLocation location))
      (LocalVariables|Settemp%20rotation (CallFunction|UpdateRoataion Rotation))
      (Math|Integer|IncrementInt (Variables|Default|GetCurrentRecursion)
        (:%20%20
          (CallFunction|UpdateScenecaptureRecusive# (LocalVariables|GetTemporaryLocation) (LocalVariables|Gettemp%20rotation))
          (Transformation|SetWorldLocationAndRotation (Variables|UwU_Portal_C|GetPortalCamera (Variables|Default|GetLinked%20Portal)) (LocalVariables|GetTemporaryLocation) (LocalVariables|Gettemp%20rotation) false false)
          (Rendering|SceneCapture|CaptureScene (Variables|UwU_Portal_C|GetPortalCamera (Variables|Default|GetLinked%20Portal)) :!class /Script/Engine.SceneCaptureComponent2D)))
      (else
        (Transformation|SetWorldLocationAndRotation (Variables|UwU_Portal_C|GetPortalCamera (Variables|Default|GetLinked%20Portal)) (CallFunction|UpdateLocation location) (CallFunction|UpdateRoataion Rotation) false false)
        (Rendering|SetVisibility (Variables|Default|GetPortal) false false)
        (Rendering|SceneCapture|CaptureScene (Variables|UwU_Portal_C|GetPortalCamera (Variables|Default|GetLinked%20Portal)) :!class /Script/Engine.SceneCaptureComponent2D)
        (Rendering|SetVisibility (Variables|Default|GetPortal) true false)))))