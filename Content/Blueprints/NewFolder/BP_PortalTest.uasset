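; Linked portal actor that shows a see-through view of its partner and teleports the player through.
; The primary links both portals and assigns render targets and materials by Pair.
; While enabled, Tick sizes the target to the viewport, mirrors the camera onto the partner's capture and updates clip planes.
; Overlap plus a predicted-position dot test triggers Teleport, remapping rotation and boosted velocity; the Teleportable-object branch only ever receives a null Object.
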(event OnComponentBeginOverlap(Box)
  (params (OverlappedComponent :type Primitive%20Component%20Object%20Reference) (OtherActor :type Actor%20Object%20Reference) (OtherComp :type Primitive%20Component%20Object%20Reference) (OtherBodyIndex :type Integer) (bFromSweep :type Boolean) (SweepResult :type Hit%20Result%20Structure%20%28by%20ref%29))
  (Utilities|Casting|CastToBP_FirstPersonCharacter OtherActor
    (:then
      (Variables|Default|SetIsOverlaping true)
      (Variables|Default|SetPorO true))
    (:CastFailed
      (if (Utilities|DoesObjectImplementInterface OtherActor "/Game/Interfaces/BPI_Teleportable.BPI_Teleportable_C")
        (Variables|Default|SetIsOverlaping true)
        (Variables|Default|SetObject 0)
        (Variables|Default|SetPorO false)))))

(event OnComponentEndOverlap(Box)
  (params (OverlappedComponent :type Primitive%20Component%20Object%20Reference) (OtherActor :type Actor%20Object%20Reference) (OtherComp :type Primitive%20Component%20Object%20Reference) (OtherBodyIndex :type Integer))
  (Utilities|Casting|CastToBP_FirstPersonCharacter OtherActor
    (:then
      (Variables|Default|SetIsOverlaping false)
      (Variables|Default|SetPorO true))
    (:CastFailed
      (if (Utilities|DoesObjectImplementInterface OtherActor "/Game/Interfaces/BPI_Teleportable.BPI_Teleportable_C")
        (Variables|Default|SetIsOverlaping false)
        (Variables|Default|SetObject 0)
        (Variables|Default|SetPorO false)))))

(event EventBeginPlay
  (bind _asbp_first_person_character (Utilities|Casting|CastToBP_FirstPersonCharacter (Game|GetPlayerCharacter 0)))
  (Variables|Default|SetAs%20BP%20First%20Person%20Character _asbp_first_person_character))

(event Collision|EventActorBeginOverlap
  (params (OtherActor :type Actor%20Object%20Reference)))

(event EventTick
  (params (DeltaSeconds :type Float%20%28single-precision%29))
  (if (Variables|Default|GetIsEnabled)
    (CallFunction|UpdateRednerTarget)))

(fn ConstructionScript
  (CallFunction|PrimarySetup))

(fn PrimarySetup
  (bind _pair (Variables|Default|GetPair))
  (if (and (Variables|Default|GetIsPrimary) (Variables|Default|GetIsEnabled))
    (CallFunction|SetupRenderTarget (Utilities|Select :Index _pair :Option%200 "/Game/Blueprints/NewFolder/RT_Portal1.RT_Portal1" :Option%201 "/Game/Blueprints/NewFolder/RT_Portal3.RT_Portal3" :Option%202 "/Game/Blueprints/NewFolder/RT_Portal5.RT_Portal5" :Option%203 "/Game/Blueprints/NewFolder/RT_Portal7.RT_Portal7"))
    (Variables|BP_PortalTest_C|SetLinked%20Portal (Variables|Default|GetLinked%20Portal) self)
    (CallFunction|SetupRenderTarget (Variables|Default|GetLinked%20Portal) (Utilities|Select :Index _pair :Option%200 "/Game/Blueprints/NewFolder/RT_Portal2.RT_Portal2" :Option%201 "/Game/Blueprints/NewFolder/RT_Portal4.RT_Portal4" :Option%202 "/Game/Blueprints/NewFolder/RT_Portal6.RT_Portal6" :Option%203 "/Game/Blueprints/NewFolder/RT_Portal8.RT_Portal8"))))

(fn SetupRenderTarget
  (params (RenderTarget :type Texture%20Render%20Target%202D%20Object%20Reference))
  (Variables|/Script/Engine.SceneCaptureComponent2D|SetTextureTarget (Variables|Default|GetSceneCaptureComponent2D) RenderTarget)
  (Rendering|Material|SetMaterial (Variables|Default|GetPlane) 0 (Utilities|Select :Index (Variables|Default|GetPair) :Option%200 (select (Variables|Default|GetIsPrimary) "/Game/Blueprints/NewFolder/M_Portal_2.M_Portal_2" "/Game/Blueprints/NewFolder/M_Portal_1.M_Portal_1") :Option%201 (select (Variables|Default|GetIsPrimary) "/Game/Blueprints/NewFolder/M_Portal_4.M_Portal_4" "/Game/Blueprints/NewFolder/M_Portal_3.M_Portal_3") :Option%202 (select (Variables|Default|GetIsPrimary) "/Game/Blueprints/NewFolder/M_Portal_6.M_Portal_6" "/Game/Blueprints/NewFolder/M_Portal_5.M_Portal_5") :Option%203 (select (Variables|Default|GetIsPrimary) "/Game/Blueprints/NewFolder/M_Portal_8.M_Portal_8" "/Game/Blueprints/NewFolder/M_Portal_7.M_Portal_7"))))

(fn UpdateRednerTarget
  (bind _returnvalue (Viewport|GetViewportSize))
  (bind _arrow (Variables|Default|GetArrow))
  (bind _as_bp_first_person_character (Variables|Default|GetAs%20BP%20First%20Person%20Character))
  (Rendering|ResizeRenderTarget2D (Variables|/Script/Engine.SceneCaptureComponent2D|GetTextureTarget (Variables|Default|GetSceneCaptureComponent2D)) (Math|Float|Truncate (.x _returnvalue)) (Math|Float|Truncate (.y _returnvalue)))
  (bind _as_bp_first_person_character_2 (Variables|Default|GetAs%20BP%20First%20Person%20Character)
    (:then
      (Transformation|SetRelativeLocationAndRotation (Variables|BP_PortalTest_C|GetSceneCaptureComponent2D (Variables|Default|GetLinked%20Portal)) (.location (Math|Transform|MakeRelativeTransform (Transformation|GetWorldTransform (Variables|/Game/FirstPerson/Blueprints/BP_FirstPersonCharacter.BP_FirstPersonCharacter_C|GetFirstPersonCamera _as_bp_first_person_character_2)) (Transformation|GetWorldTransform (Variables|Default|GetBackfacing)))) (.rotation (Math|Transform|MakeRelativeTransform (Transformation|GetWorldTransform (Variables|/Game/FirstPerson/Blueprints/BP_FirstPersonCharacter.BP_FirstPersonCharacter_C|GetFirstPersonCamera _as_bp_first_person_character_2)) (Transformation|GetWorldTransform (Variables|Default|GetBackfacing)))) false false)
      (Variables|/Script/Engine.SceneCaptureComponent2D|SetClipPlaneBase (Variables|Default|GetSceneCaptureComponent2D) (Transformation|GetWorldLocation (Variables|BP_PortalTest_C|GetArrow (Variables|Default|GetLinked%20Portal))))
      (Variables|/Script/Engine.SceneCaptureComponent2D|SetClipPlaneNormal (Variables|Default|GetSceneCaptureComponent2D) (Math|Vector|GetForwardVector (Variables|Default|GetArrow)))
      (if (Variables|Default|GetIsOverlaping)
        (if (>= (Math|Vector|DotProduct (Math|Vector|GetForwardVector _arrow) (Math|Vector|Normalize (- (Transformation|GetWorldLocation _arrow) (+ (Transformation|GetActorLocation _as_bp_first_person_character) (* (+ (Transformation|GetVelocity _as_bp_first_person_character) "2.000000,0.000000,0.000000") (Utilities|Time|GetWorldDeltaSeconds)))))) 0.0)
          (CallFunction|Teleport))))
    (:else)))

(fn Teleport
  (bind _object (Variables|Default|GetObject))
  (bind _as_bp_first_person_character (Variables|Default|GetAs%20BP%20First%20Person%20Character))
  (bind _arrow (Variables|Default|GetArrow))
  (bind _linked_portal (Variables|Default|GetLinked%20Portal))
  (bind _arrow_2 (Variables|Default|GetArrow))
  (bind _linked_portal_2 (Variables|Default|GetLinked%20Portal))
  (bind _returnvalue (Transformation|GetWorldTransform _arrow))
  (bind _returnvalue_2 (Transformation|GetActorRotation _object))
  (bind _returnvalue_3 (Transformation|GetWorldTransform _arrow_2))
  (bind _returnvalue_4 (Pawn|GetController _as_bp_first_person_character))
  (bind _backfacing (Variables|BP_PortalTest_C|GetBackfacing _linked_portal))
  (bind _backfacing_2 (Variables|BP_PortalTest_C|GetBackfacing _linked_portal_2))
  (bind _returnvalue_5 (Math|Transform|InverseTransformRotation _returnvalue _returnvalue_2))
  (bind _returnvalue_6 (Transformation|GetWorldTransform _backfacing_2))
  (bind _returnvalue_7 (Pawn|GetControlRotation _returnvalue_4 :!class /Script/Engine.Controller))
  (bind _returnvalue_8 (Transformation|GetWorldTransform _backfacing))
  (bind _returnvalue_9 (Math|Transform|TransformRotation _returnvalue_8 _returnvalue_5))
  (bind _returnvalue_10 (Math|Transform|InverseTransformRotation _returnvalue_3 _returnvalue_7))
  (bind _returnvalue_11 (Math|Transform|TransformRotation _returnvalue_6 _returnvalue_10))
  (if (Variables|Default|GetPorO)
    (Variables|Default|SetL-Velocity (* (Math|Transform|TransformDirection (Transformation|GetWorldTransform (Variables|BP_PortalTest_C|GetBackfacing (Variables|Default|GetLinked%20Portal))) (Math|Transform|InverseTransformDirection (Transformation|GetWorldTransform (Variables|Default|GetArrow)) (Transformation|GetVelocity (Variables|Default|GetAs%20BP%20First%20Person%20Character)))) "1.400000,1.400000,1.400000"))
    (Variables|Default|SetL-Position (Math|Transform|TransformLocation (Transformation|GetWorldTransform (Variables|BP_PortalTest_C|GetBackfacing (Variables|Default|GetLinked%20Portal))) "0, 0, 0"))
    (Variables|Default|SetL-Rotation (Math|Rotator|MakeRotator 0.0 (.pitch _returnvalue_11) (.yaw _returnvalue_11)))
    (Pawn|SetControlRotation (Pawn|GetController (Variables|Default|GetAs%20BP%20First%20Person%20Character)) (Variables|Default|GetL-Rotation))
    (Transformation|SetActorLocationAndRotation (Variables|Default|GetAs%20BP%20First%20Person%20Character) (Variables|Default|GetL-Position) (Variables|Default|GetL-Rotation))
    (Variables|/Script/Engine.MovementComponent|SetVelocity (Variables|/Script/Engine.Character|GetCharacterMovement (Variables|Default|GetAs%20BP%20First%20Person%20Character)) (Variables|Default|GetL-Velocity))
    (if (Variables|Default|GetisSize)
      _)
    (else
      (Variables|Default|SetL-Velocity (* (Math|Transform|TransformDirection (Transformation|GetWorldTransform (Variables|BP_PortalTest_C|GetBackfacing (Variables|Default|GetLinked%20Portal))) (Math|Transform|InverseTransformDirection (Transformation|GetWorldTransform (Variables|Default|GetArrow)) (Transformation|GetVelocity (Variables|Default|GetObject)))) "1.400000,1.400000,1.400000"))
      (Variables|Default|SetL-Position (Math|Transform|TransformLocation (Transformation|GetWorldTransform (Variables|BP_PortalTest_C|GetBackfacing (Variables|Default|GetLinked%20Portal))) "0, 0, 0"))
      (bind _output_get (Variables|Default|SetL-Rotation (Math|Rotator|MakeRotator 0.0 (.pitch _returnvalue_9) (.yaw _returnvalue_9))))
      (Transformation|SetActorLocationAndRotation (Variables|Default|GetObject) (Variables|Default|GetL-Position) _output_get)
      (if (Variables|Default|GetisSize)
        _))))